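; AI controller for the melee enemy that runs the BT_Enemy behavior tree and feeds its blackboard.
; On BeginPlay it starts the tree and caches the controlled BP_EnemyMelee pawn.
; AI perception updates toggle SeesPlayer, writing the Player key when an actor tagged Player is sensed.
; Every tick it sets IsDead to the inverse of the pawn's CanMove flag.
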(event `self.ReceiveBeginPlay`
  ;[1 1 1] On Possess
  (`self.RunBehaviorTree` "/Game/Models/AI/Blueprints/BT_Enemy.BT_Enemy")
  (bind _asbp_enemy_melee (cast `/Game/Models/AI/Blueprints/BP_EnemyMelee` (`self.K2_GetPawn`)))
  (set `self.As BP Enemy Melee` _asbp_enemy_melee))

(event `self.AIPerception.OnTargetPerceptionUpdated`
  (params (Actor :type "Actor Object Reference") (Stimulus :type "AIStimulus Structure"))
  (bind _blackboard (`self.Blackboard`))
  (if (and (`self.ActorHasTag` Actor "Player") (`.bSuccessfullySensed` (break `AIStimulus` Stimulus)))
    (`BlackboardComponent.SetValueAsObject` _blackboard (`self.Player`) null)
    (`BlackboardComponent.SetValueAsBool` _blackboard (`self.SeesPlayer`) true)
    (else
      (`BlackboardComponent.SetValueAsBool` (`self.Blackboard`) (`self.SeesPlayer`) false))))

(event `self.ReceiveTick`
  (params (DeltaSeconds :type "Float (single-precision)"))
  (`BlackboardComponent.SetValueAsBool` (`self.Blackboard`) (`self.IsDead`) (not (`/Game/Models/AI/Blueprints/BP_EnemyMelee.CanMove` (`self.As BP Enemy Melee`)))))

(fn `UserConstructionScript`)