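; Melee AI enemy character that spawns a sword on its hand socket, attacks with slash montages and dies when HP runs out.
; EnemyAttack plays the slash on a cooldown; CheckHit applies damage when the sword socket is within range of the cached target.
; GetNearestEnemy sphere-traces for pawns, but its self-equal distance comparison keeps the last hit, not the nearest.
; Pawn sensing is empty and the move-to-player node is unconnected.
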(event `SetSpeed`
  (params (Speed :type "Float (double-precision)" :default 100.0))
  ;[1 1 1] Set Speed
  (set `CharacterMovementComponent.MaxWalkSpeed` Speed (`self.CharacterMovement`)))

(event `self.ReceiveBeginPlay`
  ;[1 1 1] Begin Play
  (`|ExecutionSequence`
    (:`then_0`
      (set `self.PlayerRef` (`GameplayStatics.GetPlayerPawn` 0)))
    (:`then_1`
      (bind _asexo_gray_skeleton_anim_blueprint (cast `/Game/Models/AI/exo_gray_Skeleton_AnimBlueprint` (`SkeletalMeshComponent.GetAnimInstance` (`self.Mesh`))))
      (set `self.AnimBP` _asexo_gray_skeleton_anim_blueprint))
    (:`then_2`
      (`self.Spawn Weapon`))
    (:`then_3`
      (set `self.HP` (`self.MaxHP`)))))

(event `self.PawnSensing.OnSeePawn`
  (params (Pawn :type "Pawn Object Reference"))
  ;[1 1 1] See Pawn
)

(event `Spawn Weapon`
  ;[1 1 1] Spawn weapon
  (bind _returnvalue (`|SpawnActorFromClass` "/Game/InfinityBladeWeapons/Weapons/Dual_Blade/Dual_Blade_Tech/BP_EnemySword.BP_EnemySword_C" (`SceneComponent.GetSocketTransform` (`self.Mesh`) "SwordSocket" "RTS_World") "Undefined" "OverrideRootScale" null null))
  (bind _output_get (set `self.Sword` _returnvalue))
  (`self.K2_AttachToComponent` _output_get (`self.Mesh`) "SwordSocket" "SnapToTarget" "SnapToTarget" "SnapToTarget" true))

(event `EnemyAttack`
  ;[1 1 1] Enemy Attack
  (if (`self.CanMove`)
    (`/Engine/EditorBlueprintResources/StandardMacros.DoOnce` false :!label _label
      (:`Completed`
        (`AnimInstance.Montage_Play` (`self.AnimBP`) "/Game/Models/AI/Animations/Sword_And_Shield_Slash_Montage.Sword_And_Shield_Slash_Montage" 1.0 "MontageLength" 0.0 true)
        (set `self.AttackDamage` 10.0)
        (`KismetSystemLibrary.Delay` 3.0)
        (goto _label :!via `Reset`)))))

(event `CheckHit`
  (bind _nearestenemy (`self.NearestEnemy`))
  (bind _nearestenemy_2 (`self.NearestEnemy`))
  (`/Engine/EditorBlueprintResources/StandardMacros.IsValid` _nearestenemy
    (:`Is Valid`
      _)
    (:`Is Not Valid`
      (`self.Get Nearest Enemy`)))
  (`/Engine/EditorBlueprintResources/StandardMacros.IsValid` _nearestenemy
    (:`Is Valid`
      (if (< (`KismetMathLibrary.VSize` (- (`SceneComponent.GetSocketLocation` (`Actor.RootComponent` (`self.Sword`)) "CheckHitSocket") (`self.K2_GetActorLocation` _nearestenemy))) (`self.HitRange`))
        (`KismetSystemLibrary.PrintString` "Hit")
        (`|PlayMontage` (`self.GetComponentByClass` _nearestenemy_2 "/Script/Engine.SkeletalMeshComponent")
          (:`then`
            (`GameplayStatics.ApplyDamage` _nearestenemy_2 (`self.AttackDamage`) null self)
            (`KismetSystemLibrary.Delay` 0.3)))))))

(event `self.ReceiveAnyDamage`
  (params (Damage :type "Float (single-precision)") (DamageType :type "DamageType Object Reference") (InstigatedBy :type "Controller Object Reference") (DamageCauser :type "Actor Object Reference"))
  (if (!= DamageCauser "BP_EnemyMelee")
    (bind _output_get (set `self.HP` (- (`self.HP`) Damage)))
    (if (<= _output_get 0.0)
      (set `self.CanMove` false)
      (`AnimInstance.Montage_Play` (`self.AnimBP`) "/Game/Models/AI/Animations/Sword_And_Shield_Death_Montage.Sword_And_Shield_Death_Montage" 1.0 "MontageLength" 0.0 true)
      (`KismetSystemLibrary.Delay` 10.0)
      (`self.K2_DestroyActor`))))

(fn `Get Nearest Enemy`
  (returns (NearestEnemy :type "Actor Object Reference"))
  (bind _returnvalue (`self.K2_GetActorLocation`))
  (bind _nearestenemy (`self.NearestEnemy`))
  (bind _outhits (`KismetSystemLibrary.SphereTraceMultiForObjects` _returnvalue (`KismetMathLibrary.MakeVector` (+ (.x _returnvalue) 0.1) (+ (.y _returnvalue) 0.1) (+ (.z _returnvalue) 0.1)) 300.0 (`|MakeArray` "ObjectTypeQuery3" :!type "EObjectTypeQuery Enum")))
  (for _array_element _outhits
    (`/Engine/EditorBlueprintResources/StandardMacros.IsValid` (`self.NearestEnemy`)
      (:`Is Valid`
        (if (not (< (`self.GetDistanceTo` _nearestenemy self) (`self.GetDistanceTo` self _nearestenemy)))
          (set `self.NearestEnemy` (`.HitActor` (`GameplayStatics.BreakHitResult` _array_element)) :!label _label)))
      (:`Is Not Valid`
        (goto _label))))
  (return (`self.NearestEnemy`)))

(fn `UserConstructionScript`)