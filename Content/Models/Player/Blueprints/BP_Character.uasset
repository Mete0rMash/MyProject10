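; Player character for melee combat with a sword and paired gauntlets, plus movement, HUD health and death.
; Weapons spawn on body sockets and move to hand sockets on equip.
; Attacks auto-turn toward the nearest enemy; buffered input chains gauntlet light and sword heavy combos with scaling damage.
; CheckHit uses socket distance to the nearest enemy instead of collision; lock-on yaws toward the target but is marked broken.
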(event `InputAxis|TurnCamera`
  (params (AxisValue :type "Float (single-precision)"))
  ;[1 1 1] Movement
  (if (`self.CanControlCamera`)
    (`self.AddControllerYawInput` AxisValue)))

(event `InputAxis|Move_Forward`
  (params (AxisValue :type "Float (single-precision)"))
  ;[1 1 1] Movement
  (if (`self.MovementOn`)
    (`self.AddMovementInput` (`KismetMathLibrary.GetForwardVector` (`KismetMathLibrary.MakeRotator` 0.0 0.0 (.yaw (`self.GetControlRotation`)))) AxisValue)))

(event `InputAxis|Move_Sides`
  (params (AxisValue :type "Float (single-precision)"))
  ;[1 1 1] Movement
  (if (`self.MovementOn`)
    (`self.AddMovementInput` (`KismetMathLibrary.GetRightVector` (`KismetMathLibrary.MakeRotator` 0.0 0.0 (.yaw (`self.GetControlRotation`)))) AxisValue)))

(event `Movement`
  (params (`On / Off` :type Boolean))
  ;[1 1 1] Movement
  (set `self.MovementOn` `On / Off`))

(event `SpawnSword`
  ;[1 1 1] Spawn Weapons
  (bind _returnvalue (`|SpawnActorFromClass` "/Game/Models/Weapons/Sword/BP_Sword.BP_Sword_C" (`SceneComponent.GetSocketTransform` (`self.Mesh`) "SpineSocket" "RTS_World") "Undefined" "OverrideRootScale" null null))
  (bind _output_get (set `self.Sword` _returnvalue))
  (`self.K2_AttachToComponent` _output_get (`self.Mesh`) "SpineSocket" "SnapToTarget" "SnapToTarget" "SnapToTarget" true))

(event `SpawnGaunt`
  (bind _mesh (`self.Mesh`))
  ;[1 1 1] Spawn Weapons
  (bind _returnvalue (`|SpawnActorFromClass` "/Game/Models/Weapons/Gauntlet/BP_Gaunt1.BP_Gaunt1_C" (`SceneComponent.GetSocketTransform` _mesh "HipsSocket" "RTS_World") "Undefined" "OverrideRootScale" null null))
  (bind _output_get (set `self.Gaunt1` _returnvalue))
  (`self.K2_AttachToComponent` _output_get (`self.Mesh`) "HipsSocket" "SnapToTarget" "SnapToTarget" "SnapToTarget" true)
  (bind _returnvalue_2 (`|SpawnActorFromClass` "/Game/Models/Weapons/Gauntlet/BP_Gaunt2.BP_Gaunt2_C" (`SceneComponent.GetSocketTransform` _mesh "HipsSocket2" "RTS_World") "Undefined" "OverrideRootScale" null null))
  (bind _output_get_2 (set `self.Gaunt2` _returnvalue_2))
  (`self.K2_AttachToComponent` _output_get_2 (`self.Mesh`) "HipsSocket2" "SnapToTarget" "SnapToTarget" "SnapToTarget" true))

(event `InputAction|Weapon1`
  (params (Key :type "Key Structure"))
  (bind _animref (`self.AnimRef`))
  (bind _animref_2 (`self.AnimRef`))
  ;[1 1 1] Change Weapon Status
  (:`Pressed`
    (if (and (`/Game/Models/Player/Blueprints/Anim_Character.IsWeaponActive` _animref) (!= (`self.WeaponType`) 2))
      (set `/Game/Models/Player/Blueprints/Anim_Character.IsWeaponActive` false _animref)
      (set `self.WeaponType` 0)
      (`AnimInstance.Montage_Play` _animref_2 "/Game/Models/Player/Animations/A_Soldier_Standing_Disarm_Over_Shoulder_Montage.A_Soldier_Standing_Disarm_Over_Shoulder_Montage" 1.0 "MontageLength" 0.0 true)
      (`KismetSystemLibrary.Delay` 1.0)
      (`self.K2_AttachToComponent` (`self.Sword`) (`self.Mesh`) "SpineSocket" "SnapToTarget" "SnapToTarget" "SnapToTarget" true)
      (else
        (set `/Game/Models/Player/Blueprints/Anim_Character.IsWeaponActive` true _animref)
        (set `self.WeaponType` 1)
        (`AnimInstance.Montage_Play` _animref_2 "/Game/Models/Player/Animations/A_Soldier_Unarmed_Equip_Over_Shoulder_Montage.A_Soldier_Unarmed_Equip_Over_Shoulder_Montage" 1.0 "MontageLength" 0.0 true)
        (`KismetSystemLibrary.Delay` 1.0)
        (`self.K2_AttachToComponent` (`self.Sword`) (`self.Mesh`) "SwordSocket" "SnapToTarget" "SnapToTarget" "SnapToTarget" true)))))

(event `InputAction|Weapon2`
  (params (Key :type "Key Structure"))
  (bind _animref (`self.AnimRef`))
  (bind _animref_2 (`self.AnimRef`))
  ;[1 1 1] Change Weapon Status
  (:`Pressed`
    (if (and (`/Game/Models/Player/Blueprints/Anim_Character.IsWeaponActive` _animref) (!= (`self.WeaponType`) 1))
      (set `/Game/Models/Player/Blueprints/Anim_Character.IsWeaponActive` false _animref)
      (set `self.WeaponType` 0)
      (`AnimInstance.Montage_Play` _animref_2 "/Game/Models/Player/Animations/A_Soldier_Standing_Disarm_Underarm_Montage.A_Soldier_Standing_Disarm_Underarm_Montage" 1.0 "MontageLength" 0.0 true)
      (`KismetSystemLibrary.Delay` 1.0)
      (`self.K2_AttachToComponent` (`self.Gaunt1`) (`self.Mesh`) "HipsSocket" "SnapToTarget" "SnapToTarget" "SnapToTarget" true)
      (`self.K2_AttachToComponent` (`self.Gaunt2`) (`self.Mesh`) "HipsSocket2" "SnapToTarget" "SnapToTarget" "SnapToTarget" true)
      (else
        (set `/Game/Models/Player/Blueprints/Anim_Character.IsWeaponActive` true _animref)
        (set `self.WeaponType` 2)
        (`AnimInstance.Montage_Play` _animref_2 "/Game/Models/Player/Animations/A_Soldier_Unarmed_Equip_Underarm_Montage.A_Soldier_Unarmed_Equip_Underarm_Montage" 1.0 "MontageLength" 0.0 true)
        (`KismetSystemLibrary.Delay` 1.0)
        (`self.K2_AttachToComponent` (`self.Gaunt1`) (`self.Mesh`) "GauntSocket" "SnapToTarget" "SnapToTarget" "SnapToTarget" true)
        (`self.K2_AttachToComponent` (`self.Gaunt2`) (`self.Mesh`) "GauntSocket2" "SnapToTarget" "SnapToTarget" "SnapToTarget" true)))))

(event `InputAction|PrimaryAction`
  (params (Key :type "Key Structure"))
  (bind _returnvalue (`self.K2_GetActorLocation`))
  (bind _returnvalue_2 (`self.K2_GetActorLocation`))
  (bind _capsulecomponent (`self.CapsuleComponent`))
  (bind _capsulecomponent_2 (`self.CapsuleComponent`))
  (bind _animref (`self.AnimRef`))
  (bind (_returnvalue_roll _returnvalue_pitch) (`KismetMathLibrary.BreakRotator` (`SceneComponent.K2_GetComponentRotation` _capsulecomponent)))
  (bind (_returnvalue_roll_2 _returnvalue_pitch_2) (`KismetMathLibrary.BreakRotator` (`SceneComponent.K2_GetComponentRotation` _capsulecomponent_2)))
  (bind (_returnvalue_roll_3 _returnvalue_pitch_3 _returnvalue_yaw) (`KismetMathLibrary.BreakRotator` (`KismetMathLibrary.FindLookAtRotation` _returnvalue (`self.K2_GetActorLocation` (`self.NearestEnemy`)))))
  (bind (_returnvalue_roll_4 _returnvalue_pitch_4 _returnvalue_yaw_2) (`KismetMathLibrary.BreakRotator` (`KismetMathLibrary.FindLookAtRotation` _returnvalue_2 (`self.K2_GetActorLocation` (`self.NearestEnemy`)))))
  ;[1 1 1] Light Attack
  (:`Pressed`
    (if (`/Game/Models/Player/Blueprints/Anim_Character.IsWeaponActive` (`self.AnimRef`))
      (if (`self.IsLockedOn`)
        (if (`self.IsAttacking`) :!label _label
          (set `self.CanCombo` true)
          (else
            (set `self.IsAttacking` true)
            (if (== (`self.WeaponType`) 2)
              (switch `int` (`/Game/Models/Player/Blueprints/Anim_Character.ComboCount` (`self.AnimRef`)) :!label _label_2
                (:`0`
                  (bind _output_get (set `self.AttackDamage` 10.0))
                  (set `/Game/Models/Player/Blueprints/Anim_Character.ComboCount` 1 _animref)
                  (`AnimInstance.Montage_Play` _animref "/Game/Models/Player/Animations/GauntPunching_Montage.GauntPunching_Montage" 1.0 "MontageLength" 0.0 true))
                (:`1`
                  (bind _output_get_2 (set `self.AttackDamage` (* _output_get 1.2)))
                  (set `/Game/Models/Player/Blueprints/Anim_Character.ComboCount` 2 _animref)
                  (`AnimInstance.Montage_Play` _animref "/Game/Models/Player/Animations/GauntCross_Punch_Montage.GauntCross_Punch_Montage" 1.0 "MontageLength" 0.0 true))
                (:`2`
                  (bind _output_get_3 (set `self.AttackDamage` (* _output_get_2 1.2)))
                  (set `/Game/Models/Player/Blueprints/Anim_Character.ComboCount` 3 _animref)
                  (`AnimInstance.Montage_Play` _animref "/Game/Models/Player/Animations/GauntHook_Montage.GauntHook_Montage" 1.0 "MontageLength" 0.0 true))
                (:`3`
                  (set `self.AttackDamage` (* _output_get_3 1.2))
                  (set `/Game/Models/Player/Blueprints/Anim_Character.ComboCount` 0 _animref)
                  (`AnimInstance.Montage_Play` _animref "/Game/Models/Player/Animations/GauntSurprise_Uppercut_Montage.GauntSurprise_Uppercut_Montage" 1.0 "MontageLength" 0.0 true)))
              (elif (== (`self.WeaponType`) 1)
                (set `self.AttackDamage` 10.0)
                (if (`self.IsLockedOn`)
                  (`AnimInstance.Montage_Play` (`self.AnimRef`) "/Game/Models/Player/Animations/A_Soldier_Stable_Sword_Inward_Slash_Montage.A_Soldier_Stable_Sword_Inward_Slash_Montage" 1.0 "MontageLength" 0.0 true :!label _label_3)
                  (else
                    (bind _nearestenemy (`self.Get Nearest Enemy`))
                    (`/Engine/EditorBlueprintResources/StandardMacros.IsValid` _nearestenemy
                      (:`Is Valid`
                        (`|ExecutionSequence`
                          (:`then_0`
                            (goto _label_3))
                          (:`then_1`
                            (`KismetSystemLibrary.MoveComponentTo` _capsulecomponent_2 _returnvalue_2 (`KismetMathLibrary.MakeRotator` _returnvalue_roll_2 _returnvalue_pitch_2 _returnvalue_yaw_2) false false 0.4))))
                      (:`Is Not Valid`
                        (goto _label_3)))))))))
        (else
          (bind _nearestenemy_2 (`self.Get Nearest Enemy`))
          (`/Engine/EditorBlueprintResources/StandardMacros.IsValid` _nearestenemy_2
            (:`Is Valid`
              (`|ExecutionSequence`
                (:`then_0`
                  (goto _label))
                (:`then_1`
                  (`KismetSystemLibrary.MoveComponentTo` _capsulecomponent _returnvalue (`KismetMathLibrary.MakeRotator` _returnvalue_roll _returnvalue_pitch _returnvalue_yaw)))))
            (:`Is Not Valid`
              (goto _label))))))))

(event `Combo`
  ;[1 1 1] Light Attack
  (if (`self.CanCombo`)
    (set `self.CanCombo` false)
    (goto _label_2)))

(event `ResetCombo`
  ;[1 1 1] Light Attack
  (set `/Game/Models/Player/Blueprints/Anim_Character.ComboCount` 0 (`self.AnimRef`))
  (set `self.CanComboHeavy` false)
  (set `self.CanCombo` false)
  (set `self.IsAttacking` false))

(event `InputAction|SecondaryAction`
  (params (Key :type "Key Structure"))
  (bind _returnvalue (`self.K2_GetActorLocation`))
  (bind _capsulecomponent (`self.CapsuleComponent`))
  (bind _animref (`self.AnimRef`))
  (bind (_returnvalue_roll _returnvalue_pitch) (`KismetMathLibrary.BreakRotator` (`SceneComponent.K2_GetComponentRotation` _capsulecomponent)))
  (bind (_returnvalue_roll_2 _returnvalue_pitch_2 _returnvalue_yaw) (`KismetMathLibrary.BreakRotator` (`KismetMathLibrary.FindLookAtRotation` _returnvalue (`self.K2_GetActorLocation` (`self.NearestEnemy`)))))
  ;[1 1 1] Heavy Attack
  (:`Pressed`
    (if (`/Game/Models/Player/Blueprints/Anim_Character.IsWeaponActive` (`self.AnimRef`))
      (if (`self.IsLockedOn`)
        (if (`self.IsAttacking`) :!label _label_4
          (set `self.CanComboHeavy` true)
          (else
            (set `self.IsAttacking` true)
            (if (== (`self.WeaponType`) 1)
              (switch `int` (`/Game/Models/Player/Blueprints/Anim_Character.ComboCountHeavy` (`self.AnimRef`)) :!label _label_5
                (:`0`
                  (bind _output_get (set `self.AttackDamage` 30.0))
                  (set `/Game/Models/Player/Blueprints/Anim_Character.ComboCountHeavy` 1 _animref)
                  (`AnimInstance.Montage_Play` _animref "/Game/Models/Player/Animations/A_Soldier_Standing_Melee_Attack_Kick_Ver__2_Montage.A_Soldier_Standing_Melee_Attack_Kick_Ver__2_Montage" 1.0 "MontageLength" 0.0 true))
                (:`1`
                  (set `self.AttackDamage` (* _output_get 1.5))
                  (set `/Game/Models/Player/Blueprints/Anim_Character.ComboCountHeavy` 0 _animref)
                  (`AnimInstance.Montage_Play` _animref "/Game/Models/Player/Animations/A_Soldier_Standing_Melee_Attack_Backhand_Montage.A_Soldier_Standing_Melee_Attack_Backhand_Montage" 1.0 "MontageLength" 0.0 true)))
              (else
                (`self.ResetCombo`)))))
        (else
          (bind _nearestenemy (`self.Get Nearest Enemy`))
          (`/Engine/EditorBlueprintResources/StandardMacros.IsValid` _nearestenemy
            (:`Is Valid`
              (`|ExecutionSequence`
                (:`then_0`
                  (goto _label_4))
                (:`then_1`
                  (`KismetSystemLibrary.MoveComponentTo` _capsulecomponent _returnvalue (`KismetMathLibrary.MakeRotator` _returnvalue_roll _returnvalue_pitch _returnvalue_yaw) false false 0.4))))
            (:`Is Not Valid`
              (goto _label_4))))))))

(event `ComboHeavy`
  ;[1 1 1] Heavy Attack
  (if (`self.CanComboHeavy`)
    (set `self.CanComboHeavy` false)
    (goto _label_5)))

(event `self.ReceiveBeginPlay`
  (bind _maxhp (`self.MaxHp`))
  ;[1 1 1] Start
  (`|ExecutionSequence`
    (:`then_0`
      (bind _asanim_character (cast `/Game/Models/Player/Blueprints/Anim_Character` (`SkeletalMeshComponent.GetAnimInstance` (`self.Mesh`))))
      (set `self.AnimRef` _asanim_character))
    (:`then_1`
      (`self.SpawnSword`))
    (:`then_2`
      (`self.SpawnGaunt`))
    (:`then_3`
      (bind _returnvalue (`|CreateWidget` "/Game/Blueprints/UI/HUDWidget.HUDWidget_C" (`GameplayStatics.GetPlayerController` 0)))
      (bind _output_get (set `self.HUDwidget` _returnvalue))
      (`UserWidget.AddToViewport` _output_get 0))
    (:`then_4`
      (bind _output_get_2 (set `self.HP` _maxhp))
      (`/Game/Blueprints/UI/HUDWidget.Update Health` (`self.HUDwidget`) (/ _output_get_2 _maxhp)))))

(event `Lock On`
  (params (LockedOn :type Boolean) (LockOnto :type "Actor Object Reference"))
  ;[1 1 1] Lock On (Broken)
  (if LockedOn
    (`/Engine/EditorBlueprintResources/StandardMacros.IsValid` LockOnto
      (:`Is Valid`
        (set `self.ActorLockedOn` LockOnto)
        (set `self.IsLockedOn` true)
        (set `CharacterMovementComponent.bOrientRotationToMovement` false (`self.CharacterMovement`))))
    (else
      (set `self.IsLockedOn` false)
      (set `CharacterMovementComponent.bOrientRotationToMovement` true (`self.CharacterMovement`)))))

(event `self.ReceiveTick`
  (params (DeltaSeconds :type "Float (single-precision)"))
  (bind (_returnvalue_roll _returnvalue_pitch) (`KismetMathLibrary.BreakRotator` (`self.K2_GetActorRotation`)))
  (bind _actorlockedon (`self.ActorLockedOn`))
  (bind (_returnvalue_roll_2 _returnvalue_pitch_2 _returnvalue_yaw) (`KismetMathLibrary.BreakRotator` (`KismetMathLibrary.FindLookAtRotation` (`self.K2_GetActorLocation`) (`self.K2_GetActorLocation` _actorlockedon))))
  ;[1 1 1] Lock On (Broken)
  (if (`self.IsLockedOn`)
    (`/Engine/EditorBlueprintResources/StandardMacros.IsValid` _actorlockedon
      (:`Is Valid`
        (`self.K2_SetActorRotation` (`KismetMathLibrary.MakeRotator` _returnvalue_roll _returnvalue_pitch _returnvalue_yaw))))))

(event `InputAction|Lock On`
  (params (Key :type "Key Structure"))
  ;[1 1 1] Lock On (Broken)
  (:`Pressed`
    (if (`self.IsLockedOn`)
      (set `self.CanControlCamera` true)
      (`self.Lock On` false)
      (else
        (set `self.CanControlCamera` false)
        (bind _nearestenemy (`self.Get Nearest Enemy`))
        (`self.Lock On` true _nearestenemy)))))

(event `CheckHit`
  (bind _nearestenemy (`self.NearestEnemy`))
  (bind _nearestenemy_2 (`self.NearestEnemy`))
  (bind _returnvalue (`self.K2_GetActorLocation` _nearestenemy))
  ;[1 1 1] Hit
  (`/Engine/EditorBlueprintResources/StandardMacros.IsValid` _nearestenemy
    (:`Is Valid`
      _)
    (:`Is Not Valid`
      (`self.Get Nearest Enemy`)))
  (`/Engine/EditorBlueprintResources/StandardMacros.IsValid` _nearestenemy
    (:`Is Valid`
      (if (or (< (`KismetMathLibrary.VSize` (- (`SceneComponent.GetSocketLocation` (`/Game/Models/Weapons/Sword/BP_Sword.Sword` (`self.Sword`)) "CheckHitSocket") _returnvalue)) (`self.HitRange`)) (< (`KismetMathLibrary.VSize` (- (`SceneComponent.GetSocketLocation` (`Actor.RootComponent` (`self.Gaunt1`)) "GauntSocket") _returnvalue)) (`self.HitRange`)) (< (`KismetMathLibrary.VSize` (- (`SceneComponent.GetSocketLocation` (`Actor.RootComponent` (`self.Gaunt2`)) "GauntSocket") _returnvalue)) (`self.HitRange`)) (< (`KismetMathLibrary.VSize` (- (`SceneComponent.GetSocketLocation` (`self.Mesh`) "FootSocket") _returnvalue)) (`self.HitRange`)))
        (`|PlayMontage` (`self.GetComponentByClass` _nearestenemy_2 "/Script/Engine.SkeletalMeshComponent") "/Game/Models/AI/Animations/Sword_And_Shield_Impact_Montage.Sword_And_Shield_Impact_Montage"
          (:`then`
            (`GameplayStatics.ApplyDamage` _nearestenemy_2 (`self.AttackDamage`) null self)
            (`KismetSystemLibrary.Delay` 0.3)))))))

(event `self.ReceiveAnyDamage`
  (params (Damage :type "Float (single-precision)") (DamageType :type "DamageType Object Reference") (InstigatedBy :type "Controller Object Reference") (DamageCauser :type "Actor Object Reference"))
  (bind _output_get (set `self.HP` (- (`self.HP`) Damage)))
  (`self.UpdateStats`)
  (if (<= _output_get 0.0)
    (set `self.MovementOn` false)
    (`AnimInstance.Montage_Play` (`self.AnimRef`) "/Game/Models/Player/Animations/Sword_And_Shield_Death__1__Montage.Sword_And_Shield_Death__1__Montage" 1.0 "MontageLength" 0.0 true)
    (`KismetSystemLibrary.Delay` 60.0)
    (`self.K2_DestroyActor`)))

(event `UpdateStats`
  (`/Game/Blueprints/UI/HUDWidget.Update Health` (`self.HUDwidget`) (/ (`self.HP`) (`self.MaxHp`))))

(fn `Get Nearest Enemy`
  (returns (NearestEnemy :type "Actor Object Reference"))
  (bind _returnvalue (`self.K2_GetActorLocation`))
  (bind _nearestenemy (`self.NearestEnemy`))
  (bind _outhits (`KismetSystemLibrary.SphereTraceMultiForObjects` _returnvalue (`KismetMathLibrary.MakeVector` (+ (.x _returnvalue) 0.1) (+ (.y _returnvalue) 0.1) (+ (.z _returnvalue) 0.1)) 300.0 (`|MakeArray` "ObjectTypeQuery3" :!type "EObjectTypeQuery Enum")))
  (for _array_element _outhits
    (`/Engine/EditorBlueprintResources/StandardMacros.IsValid` (`self.NearestEnemy`)
      (:`Is Valid`
        (if (not (< (`self.GetDistanceTo` _nearestenemy self) (`self.GetDistanceTo` self _nearestenemy)))
          (set `self.NearestEnemy` (`.HitActor` (`GameplayStatics.BreakHitResult` _array_element)) :!label _label)))
      (:`Is Not Valid`
        (goto _label))))
  (return (`self.NearestEnemy`)))

(fn `UserConstructionScript`)